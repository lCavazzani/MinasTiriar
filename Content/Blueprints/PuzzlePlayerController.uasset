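; Player controller that provides click-to-move and touch-to-move navigation for the pawn, with a visible mouse cursor.
; Holding the SetDestination action or a touch opens a gate, letting Tick trace under the cursor or first finger every frame.
; MoveToHitResult issues a SimpleMoveToLocation to the hit point only when it is at least MinTravelDistance from the pawn.
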(event EventBeginPlay
  (Variables|Default|SetbShowMouseCursor true))

(event EventTick
  (params (DeltaSeconds :type Float%20%28single-precision%29))
  (Utilities|FlowControl|Sequence
    (:then_0
      (Utilities|FlowControl|Gate true
        (:Exit
          (CallFunction|MovetoHitResult (.HitResult (Game|Player|GetHitResultUnderCursorbyChannel "TraceTypeQuery1" true))))))
    (:then_1
      (Utilities|FlowControl|Gate true
        (:Exit
          (CallFunction|MovetoHitResult (.HitResult (Class|PlayerController|GetHitResultUnderFingerbyChannel "Touch1" "TraceTypeQuery1" true))))))))

(event Input|ActionEvents|InputActionSetDestination
  (params (Key :type Key%20Structure :default "None"))
  (:Pressed
    (Utilities|FlowControl|Gate true) ; enters at Open
  )
  (:Released
    (Utilities|FlowControl|Gate true) ; enters at Close
  ))

(event Input|TouchEvents|InputTouch
  (params (Location :type Vector) (FingerIndex :type ETouchIndex%20Enum))
  (:Pressed
    (Utilities|FlowControl|Gate true) ; enters at Open
  )
  (:Released
    (Utilities|FlowControl|Gate true) ; enters at Close
  ))

(fn ConstructionScript)

(fn MovetoHitResult
  (params (HitResult :type Hit%20Result%20Structure))
  (bind _location (Collision|BreakHitResult HitResult))
  (if (>= (Math|Vector|VectorLength (- (Transformation|GetActorLocation (Game|Player|GetPlayerPawn 0)) _location)) (Variables|Default|GetMinTravelDistance))
    (AI|Navigation|SimpleMovetoLocation self _location)))