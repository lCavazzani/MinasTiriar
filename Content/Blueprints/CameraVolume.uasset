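; CameraVolume is a trigger actor that switches the player's view to its own camera when a PuzzleCharacter enters its box.
; On overlap it registers itself as the character's current camera and blends the first player controller's view target to itself.
; When the UseSpine flag is set, Tick moves the camera to the spline point closest to that character and rotates it to face them.
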(event OnComponentBeginOverlap(Box)
  (params (OverlappedComponent :type Primitive%20Component%20Object%20Reference) (OtherActor :type Actor%20Object%20Reference) (OtherComp :type Primitive%20Component%20Object%20Reference) (OtherBodyIndex :type Integer) (bFromSweep :type Boolean) (SweepResult :type Hit%20Result%20Structure%20%28by%20ref%29))
  (bind _self self)
  (bind _controller (Variables|Default|GetController))
  ;[1 1 1] Set correct camera volume
  (bind _aspuzzle_character (Utilities|Casting|CastToPuzzleCharacter OtherActor))
  (bind _output_get (Variables|Default|SetCharacter _aspuzzle_character))
  (Variables|/Game/Blueprints/Character/PuzzleCharacter.PuzzleCharacter_C|SetCurrent%20Camera%20 _output_get _self)
  (Utilities|IsValid _controller
    (:Is%20Valid
      (Game|Player|SetViewTargetwithBlend _controller _self 2.0 "VTBlend_Cubic" 5.0 false))))

(event EventBeginPlay
  (Variables|Default|SetController (Game|GetPlayerController 0)))

(event Collision|EventActorBeginOverlap
  (params (OtherActor :type Actor%20Object%20Reference)))

(event EventTick
  (params (DeltaSeconds :type Float%20%28single-precision%29))
  (bind _character (Variables|Default|GetCharacter))
  (bind _returnvalue (Transformation|GetActorLocation _character))
  ;[1 1 1] Camera Rotation/Location
  (if (Variables|Default|GetUseSpine)
    (Utilities|IsValid (Variables|Default|GetCharacter)
      (:Is%20Valid
        (Transformation|SetWorldLocationAndRotation (Variables|Default|GetCamera) (Spline|FindLocationClosesttoWorldLocation (Variables|Default|GetSpline) _returnvalue "World") (Math|Rotator|FindLookatRotation (Transformation|GetWorldLocation (Variables|Default|GetCamera)) _returnvalue) false false)))))

(fn ConstructionScript)